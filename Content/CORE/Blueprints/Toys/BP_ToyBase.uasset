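; Base collectible toy that the player finds by interacting, escalating the threat from the enemy with each pickup.
; BeginPlay caches the player character, whose objectives widget supplies the entry to mark via GetTextRef, which returns Item1 here.
; Interact strikes and dims that entry, speeds up the BP_EnemyCharacter and teleports it to an offset from the toy.
; The toy then destroys itself and increments the player's found-item counter, printing the total.
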(event `self.ReceiveBeginPlay`
  (bind _asbp_third_person_character (cast `/Game/ThirdPerson/Blueprints/BP_ThirdPersonCharacter` (`GameplayStatics.GetPlayerCharacter` 0)))
  (set `self.PlayerCharacter` _asbp_third_person_character))

(event `/Game/CORE/Blueprints/BPI_Interactable.Interact`
  (bind _playercharacter (`self.PlayerCharacter`))
  (bind _itemtext (`self.GetTextRef`))
  (`TextBlock.SetStrikeBrush` _itemtext (`WidgetBlueprintLibrary.MakeBrushFromTexture` "/Engine/EngineResources/AICON-Red_Low.AICON-Red"))
  (`TextBlock.SetOpacity` _itemtext 0.5)
  (bind _returnvalue (`GameplayStatics.GetActorOfClass` "/Game/ThirdPerson/Blueprints/BP_EnemyCharacter.BP_EnemyCharacter_C"))
  (`/Game/ThirdPerson/Blueprints/BP_EnemyCharacter.IncreaseMovementSpeed` _returnvalue 20.0)
  (`self.K2_SetActorLocation` _returnvalue (+ (`SceneComponent.K2_GetComponentLocation` (`self.StaticMesh`)) 300.0) false false)
  (`self.K2_DestroyActor`)
  (bind _output_get (set `/Game/ThirdPerson/Blueprints/BP_ThirdPersonCharacter.FoundItemCounter` (+ (`/Game/ThirdPerson/Blueprints/BP_ThirdPersonCharacter.FoundItemCounter` _playercharacter) 1) _playercharacter))
  (`KismetSystemLibrary.PrintString` (`KismetStringLibrary.Conv_IntToString` _output_get)))

(fn `GetTextRef`
  (returns (ItemText :type "TextBlock Object Reference"))
  (return (`/Game/CORE/Widgets/WBP_Objectives.Item1` (`/Game/ThirdPerson/Blueprints/BP_ThirdPersonCharacter.ObjectivesWidget` (`self.PlayerCharacter`)))))

(fn `UserConstructionScript`)