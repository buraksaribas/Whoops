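; BP_Thing5 is an interactable objective pickup, the fifth item on the player's objectives list, that also escalates the enemy threat.
; On Interact, it restyles the strike brush and dims the Item5 entry in the player character's objectives widget.
; It then raises the BP_EnemyCharacter's movement speed, moves that enemy to an offset from its own mesh location and destroys itself.
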(event `/Game/CORE/Blueprints/BPI_Interactable.Interact`
  (bind _asbp_third_person_character (cast `/Game/ThirdPerson/Blueprints/BP_ThirdPersonCharacter` (`GameplayStatics.GetPlayerCharacter` 0)))
  (bind _item5 (`/Game/CORE/Widgets/WBP_Objectives.Item5` (`/Game/ThirdPerson/Blueprints/BP_ThirdPersonCharacter.ObjectivesWidget` _asbp_third_person_character)))
  (`TextBlock.SetStrikeBrush` _item5 (`WidgetBlueprintLibrary.MakeBrushFromTexture` "/Engine/EngineResources/AICON-Red_Low.AICON-Red"))
  (`TextBlock.SetOpacity` _item5 0.5)
  (bind _returnvalue (`GameplayStatics.GetActorOfClass` "/Game/ThirdPerson/Blueprints/BP_EnemyCharacter.BP_EnemyCharacter_C"))
  (`/Game/ThirdPerson/Blueprints/BP_EnemyCharacter.IncreaseMovementSpeed` _returnvalue 20.0)
  (`self.K2_SetActorLocation` _returnvalue (+ (`SceneComponent.K2_GetComponentLocation` (`self.StaticMesh`)) 100.0) false false)
  (`self.K2_DestroyActor`))

(fn `UserConstructionScript`)