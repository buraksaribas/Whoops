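; BP_Gate is the level exit gate, which opens the end-game screen once the player has found all the required items.
; BeginPlay caches the third-person player character, and Tick polls its found-item counter.
; At eight items, Tick clears the lock and destroys one enemy character per frame while any remain.
; Interact prints a locked message or adds the end-game widget to the viewport.
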(event `self.ReceiveBeginPlay`
  (bind _asbp_third_person_character (cast `/Game/ThirdPerson/Blueprints/BP_ThirdPersonCharacter` (`GameplayStatics.GetPlayerCharacter` 0)))
  (set `self.PlayerCharacter` _asbp_third_person_character))

(event `/Game/CORE/Blueprints/BPI_Interactable.Interact`
  (if (`self.IsLocked`)
    (`KismetSystemLibrary.PrintString` "Locked")
    (else
      (bind _returnvalue (`|CreateWidget` "/Game/CORE/Widgets/WBP_EndGame.WBP_EndGame_C"))
      (`UserWidget.AddToViewport` _returnvalue 0))))

(event `self.ReceiveTick`
  (params (DeltaSeconds :type "Float (single-precision)"))
  (if (== (`/Game/ThirdPerson/Blueprints/BP_ThirdPersonCharacter.FoundItemCounter` (`self.PlayerCharacter`)) 8)
    (set `self.IsLocked` false)
    (bind _returnvalue (`GameplayStatics.GetActorOfClass` "/Game/ThirdPerson/Blueprints/BP_EnemyCharacter.BP_EnemyCharacter_C"))
    (`/Engine/EditorBlueprintResources/StandardMacros.IsValid` _returnvalue
      (:`Is Valid`
        (`self.K2_DestroyActor` _returnvalue)))))

(fn `UserConstructionScript`)